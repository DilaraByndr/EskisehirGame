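; Player character for ŞakaFutbolu with shared-input local two-player movement.
; Only the PlayerIndex 0 instance handles input, moving itself on P1 axes and forwarding P2 axes to the first MainChar_BP tagged Player2, looked up on each axis event.
; Movement adds input along control-yaw forward.
; Despite its name, Rotate adds sideways input using a right vector from control roll and pitch, with yaw zeroed.
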(event `InputAxis|P2_ForwardBackward`
  (params (AxisValue :type "Float (single-precision)"))
  (if (== (`self.PlayerIndex`) 0)
    (bind _outactors (`GameplayStatics.GetAllActorsOfClassWithTag` "MainChar_BP_C" "Player2"))
    (bind _asmain_char_bp (cast `/Game/ŞakaFutbolu/MainChar_BP` (`|GetArrayItem` _outactors)))
    (`self.Movement` _asmain_char_bp AxisValue)))

(event `InputAxis|P1_ForwardBackward`
  (params (AxisValue :type "Float (single-precision)"))
  (if (== (`self.PlayerIndex`) 0)
    (`self.Movement` AxisValue)))

(event `InputAxis|P2_RightLeft`
  (params (AxisValue :type "Float (single-precision)"))
  (if (== (`self.PlayerIndex`) 0)
    (bind _outactors (`GameplayStatics.GetAllActorsOfClassWithTag` "MainChar_BP_C" "Player2"))
    (bind _asmain_char_bp (cast `/Game/ŞakaFutbolu/MainChar_BP` (`|GetArrayItem` _outactors)))
    (`self.Rotate` _asmain_char_bp AxisValue)))

(event `InputAxis|P1_RightLeft`
  (params (AxisValue :type "Float (single-precision)"))
  (if (== (`self.PlayerIndex`) 0)
    (`self.Rotate` AxisValue)))

(event `Rotate`
  (params (ScaleValue :type "Float (single-precision)"))
  (`self.AddMovementInput` (`KismetMathLibrary.GetRightVector` (`KismetMathLibrary.MakeRotator` (.roll (`self.GetControlRotation`)) (.pitch (`self.GetControlRotation`)))) ScaleValue))

(event `Movement`
  (params (ScaleValue :type "Float (single-precision)"))
  (`self.AddMovementInput` (`KismetMathLibrary.GetForwardVector` (`KismetMathLibrary.MakeRotator` 0.0 0.0 (.yaw (`self.GetControlRotation`)))) ScaleValue))

(fn `UserConstructionScript`)